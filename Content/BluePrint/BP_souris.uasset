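; BP_souris is a mouse ("souris") pickup that the player collects by touching it.
; When its capsule overlaps player 0's character, it casts to BP_FirstPersonCharLudoTest, increments NombreSouris on that character's HUDInterface, calls CompteurSouris and destroys itself.
; An unconnected branch targets BP_FirstPersonCharacter with a point counter, debug print and pickup sound, and never runs.
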(event OnComponentBeginOverlap(Capsule)
  (params (OverlappedComponent :type Primitive%20Component%20Object%20Reference) (OtherActor :type Actor%20Object%20Reference) (OtherComp :type Primitive%20Component%20Object%20Reference) (OtherBodyIndex :type Integer) (bFromSweep :type Boolean) (SweepResult :type Hit%20Result%20Structure%20%28by%20ref%29))
  (bind _returnvalue (Game|GetPlayerCharacter 0))
  (if (== OtherActor _returnvalue)
    (bind _asbp_first_person_char_ludo_test (Utilities|Casting|CastToBP_FirstPersonCharLudoTest _returnvalue))
    (bind _output_get (Variables|Default|SetAs%20BP%20First%20Person%20Char%20Ludo%20Test _asbp_first_person_char_ludo_test))
    (Math|Integer|IncrementInt (Variables|/Game/HUD/HUD_interface.HUD_interface_C|GetNombre%20souris (Variables|/Game/FirstPerson/Blueprints/BP_FirstPersonCharLudoTest.BP_FirstPersonCharLudoTest_C|GetHUD_interface _output_get))
      (:%20%20
        (Default|CompteurSouris (Variables|/Game/FirstPerson/Blueprints/BP_FirstPersonCharLudoTest.BP_FirstPersonCharLudoTest_C|GetHUD_interface _output_get))
        (Actor|DestroyActor)))))

(fn ConstructionScript)