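; BP_TriggerFin is a trigger, apparently marking the end of a run, with a floating BPPawnCopa component.
; On BeginPlay, the Flotement timeline lerps that component's relative location between its start and a point higher on Z.
; When BP_FirstPersonCharacter overlaps the Box, it sets that character's PauseTimer and CompteARebour flags, then switches the player controller to UI-only input with a visible cursor.
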(event OnComponentBeginOverlap(Box)
  (params (OverlappedComponent :type Primitive%20Component%20Object%20Reference) (OtherActor :type Actor%20Object%20Reference) (OtherComp :type Primitive%20Component%20Object%20Reference) (OtherBodyIndex :type Integer) (bFromSweep :type Boolean) (SweepResult :type Hit%20Result%20Structure%20%28by%20ref%29))
  (bind _returnvalue (Game|GetPlayerController 0))
  (bind _asbp_first_person_character (Utilities|Casting|CastToBP_FirstPersonCharacter OtherActor))
  (Variables|/Game/FirstPerson/Blueprints/BP_FirstPersonCharacter.BP_FirstPersonCharacter_C|SetPause%20Timer _asbp_first_person_character true)
  (Variables|/Game/FirstPerson/Blueprints/BP_FirstPersonCharacter.BP_FirstPersonCharacter_C|SetCompte%20a%20rebour _asbp_first_person_character true)
  (Input|SetInputModeUIOnly _returnvalue 0 "DoNotLock" false)
  (Variables|/Script/Engine.PlayerController|SetbShowMouseCursor _returnvalue true))

(event EventBeginPlay
  (bind _output_get (Variables|Default|SetStart (Variables|/Script/Engine.SceneComponent|GetRelativeLocation (Variables|Default|GetBP_pawn_copa))))
  (Variables|Default|SetEnd (Math|Vector|MakeVector (.x _output_get) (.y _output_get) (+ (.z _output_get) 2e+02)))
  (bind _newtrack_0 (Timeline|Flotement PlayFromStart)
    (:Update
      (Transformation|SetRelativeLocation (Variables|Default|GetBP_pawn_copa) (Math|Vector|Lerp(Vector) (Variables|Default|GetStart) (Variables|Default|GetEnd) _newtrack_0) false false))))

(fn ConstructionScript)