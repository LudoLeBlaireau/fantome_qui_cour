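; BP_LDBlock is a resizable block, apparently for level design, whose scale is adjusted in whole steps per axis.
; Six custom events increment or decrement the X, Y or Z size variable by one.
; All six share a single SetActorScale3D call that applies the three sizes as the actor's scale, with no clamping.
; BeginPlay and the Construction Script are empty, so scale changes only when these events are called.
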(event Custom|Z%20sise%20-%201
  (Math|Integer|DecrementInt (Variables|Default|GetZ%20sise)
    (:%20%20
      (Transformation|SetActorScale3D (Math|Vector|MakeVector (Math|Conversions|ToFloat(Integer) (Variables|Default|GetX%20sise)) (Math|Conversions|ToFloat(Integer) (Variables|Default|GetY%20sise)) (Math|Conversions|ToFloat(Integer) (Variables|Default|GetZ%20sise)))))))

(event Custom|Z%20sise%20+%201
  (Math|Integer|IncrementInt (Variables|Default|GetZ%20sise)
    (:%20%20
      (Transformation|SetActorScale3D (Math|Vector|MakeVector (Math|Conversions|ToFloat(Integer) (Variables|Default|GetX%20sise)) (Math|Conversions|ToFloat(Integer) (Variables|Default|GetY%20sise)) (Math|Conversions|ToFloat(Integer) (Variables|Default|GetZ%20sise)))))))

(event Custom|Y%20sise%20-%201
  (Math|Integer|DecrementInt (Variables|Default|GetY%20sise)
    (:%20%20
      (Transformation|SetActorScale3D (Math|Vector|MakeVector (Math|Conversions|ToFloat(Integer) (Variables|Default|GetX%20sise)) (Math|Conversions|ToFloat(Integer) (Variables|Default|GetY%20sise)) (Math|Conversions|ToFloat(Integer) (Variables|Default|GetZ%20sise)))))))

(event Custom|X%20sise%20+%201
  (Math|Integer|IncrementInt (Variables|Default|GetX%20sise)
    (:%20%20
      (Transformation|SetActorScale3D (Math|Vector|MakeVector (Math|Conversions|ToFloat(Integer) (Variables|Default|GetX%20sise)) (Math|Conversions|ToFloat(Integer) (Variables|Default|GetY%20sise)) (Math|Conversions|ToFloat(Integer) (Variables|Default|GetZ%20sise)))))))

(event Custom|x%20sise%20-%201
  (Math|Integer|DecrementInt (Variables|Default|GetX%20sise)
    (:%20%20
      (Transformation|SetActorScale3D (Math|Vector|MakeVector (Math|Conversions|ToFloat(Integer) (Variables|Default|GetX%20sise)) (Math|Conversions|ToFloat(Integer) (Variables|Default|GetY%20sise)) (Math|Conversions|ToFloat(Integer) (Variables|Default|GetZ%20sise)))))))

(event Custom|Y%20sise%20+%201
  (Math|Integer|IncrementInt (Variables|Default|GetY%20sise)
    (:%20%20
      (Transformation|SetActorScale3D (Math|Vector|MakeVector (Math|Conversions|ToFloat(Integer) (Variables|Default|GetX%20sise)) (Math|Conversions|ToFloat(Integer) (Variables|Default|GetY%20sise)) (Math|Conversions|ToFloat(Integer) (Variables|Default|GetZ%20sise)))))))

(event EventBeginPlay)

(fn ConstructionScript)