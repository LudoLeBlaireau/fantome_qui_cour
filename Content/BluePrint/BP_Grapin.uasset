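; BP_Grapin is a grapple point that offers itself to the first-person character inside its Range trigger.
; Entering or leaving Range toggles CanInteract, swaps the Grapin material and calls CanGrapin on the character with the location.
; The Delay event starts a two-second cooldown that disables the point.
; Flags track players staying in or entering Range during the cooldown, so the point re-offers itself when it ends.
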(event OnComponentBeginOverlap(Range)
  (params (OverlappedComponent :type Primitive%20Component%20Object%20Reference) (OtherActor :type Actor%20Object%20Reference) (OtherComp :type Primitive%20Component%20Object%20Reference) (OtherBodyIndex :type Integer) (bFromSweep :type Boolean) (SweepResult :type Hit%20Result%20Structure%20%28by%20ref%29))
  (bind _asbp_first_person_character (Utilities|Casting|CastToBP_FirstPersonCharacter OtherActor))
  (bind _output_get (Variables|Default|SetBP%20First%20Person%20Character _asbp_first_person_character))
  (if (Variables|Default|Getwate)
    (Variables|Default|SetEntré%20pendant%20delay true)
    (else
      (Variables|Default|Setcan%20interact true)
      (CallFunction|ChangeColor)
      (Default|CanGrapin _output_get true (Transformation|GetWorldLocation (Variables|Default|GetGrapin)) self))))

(event OnComponentEndOverlap(Range)
  (params (OverlappedComponent :type Primitive%20Component%20Object%20Reference) (OtherActor :type Actor%20Object%20Reference) (OtherComp :type Primitive%20Component%20Object%20Reference) (OtherBodyIndex :type Integer))
  (Utilities|Casting|CastToBP_FirstPersonCharacter OtherActor)
  (Variables|Default|Setcan%20interact false)
  (Variables|Default|SetToujours%20dans%20trigger false)
  (if (Variables|Default|GetEntré%20pendant%20delay)
    (Variables|Default|SetEntré%20pendant%20delay false)
    (else
      (CallFunction|ChangeColor)
      (Default|CanGrapin (stale OnComponentBeginOverlap(Range) _output_get) false "0, 0, 0"))))

(event Custom|Change%20color
  ;[0.3722 0.9271 0.1497] Change color
  (Rendering|Material|SetMaterial (Variables|Default|GetGrapin) 0 (select (Variables|Default|Getcan%20interact) "/Engine/MapTemplates/Materials/BasicAsset03.BasicAsset03" "/Engine/MapTemplates/Materials/BasicAsset01.BasicAsset01")))

(event Custom|Delay
  (Variables|Default|Setcan%20interact false)
  (Variables|Default|Setwate true)
  (Variables|Default|SetToujours%20dans%20trigger true)
  (CallFunction|ChangeColor)
  (Utilities|FlowControl|Delay 2.0)
  (Variables|Default|Setwate false)
  (if (Variables|Default|GetToujours%20dans%20trigger)
    (Variables|Default|Setcan%20interact true :!label _label)
    (CallFunction|ChangeColor)
    (Default|CanGrapin (Variables|Default|GetBP%20First%20Person%20Character) true (Transformation|GetWorldLocation (Variables|Default|GetGrapin)) self)
    (elif (Variables|Default|GetEntré%20pendant%20delay)
      (goto _label))))

(event EventBeginPlay)

(fn ConstructionScript)