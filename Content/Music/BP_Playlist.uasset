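; Music playlist Blueprint that plays the tracks in MusicPlaylist as 2D sounds in shuffled order, starting on BeginPlay.
; Each track fades in, prints its name and is removed from a temporary copy of the playlist, with its audio-finished event triggering the next.
; Once every track has been started, the copy is refilled and reshuffled.
; The F key stops the current track.
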(event Custom|Play_track
  (bind _returnvalue (Audio|SpawnSound2D (Utilities|Array|Get(acopy) (Variables|Default|GetTemp_playlist)) 1.0 1.0 0.0 0))
  (Audio|Components|Audio|FadeIn _returnvalue 1.5 1.0 0.0 "Linear" :!class /Script/Engine.AudioComponent)
  (bind _output_get (Variables|Default|SetCurrent_track _returnvalue))
  (EventDispatchers|BindEventtoOnAudioFinished _output_get (delegate Custom|OnAudioFinished_Event_0))
  (Development|PrintString (Utilities|GetDisplayName (Variables|/Script/Engine.AudioComponent|GetSound (Variables|Default|GetCurrent_track))))
  (Utilities|Array|RemoveIndex (Variables|Default|GetTemp_playlist))
  (Math|Integer|IncrementInt (Variables|Default|GetTracks_played)
    (:%20%20
      (if (== (Utilities|Array|Length (Variables|Default|GetMusic_playlist)) (Variables|Default|GetTracks_played))
        (Variables|Default|SetTemp_playlist (Variables|Default|GetMusic_playlist))
        (Utilities|Array|Shuffle (Variables|Default|GetTemp_playlist))
        (Variables|Default|SetTracks_played 0)))))

(event Custom|OnAudioFinished_Event_0
  (CallFunction|PlayTrack))

(event EventBeginPlay
  (Variables|Default|SetTemp_playlist (Variables|Default|GetMusic_playlist))
  (Utilities|Array|Shuffle (Variables|Default|GetTemp_playlist))
  (bind _returnvalue (Audio|SpawnSound2D (Utilities|Array|Get(acopy) (Variables|Default|GetTemp_playlist)) 1.0 1.0 0.0 0))
  (Audio|Components|Audio|FadeIn _returnvalue 1.5 1.0 0.0 "Linear" :!class /Script/Engine.AudioComponent)
  (bind _output_get (Variables|Default|SetCurrent_track _returnvalue))
  (EventDispatchers|BindEventtoOnAudioFinished _output_get (delegate Custom|OnAudioFinished_Event_0))
  (Development|PrintString (Utilities|GetDisplayName (Variables|/Script/Engine.AudioComponent|GetSound (Variables|Default|GetCurrent_track))))
  (Utilities|Array|RemoveIndex (Variables|Default|GetTemp_playlist))
  (Math|Integer|IncrementInt (Variables|Default|GetTracks_played)
    (:%20%20
      (if (== (Utilities|Array|Length (Variables|Default|GetMusic_playlist)) (Variables|Default|GetTracks_played))
        (Variables|Default|SetTemp_playlist (Variables|Default|GetMusic_playlist))
        (Utilities|Array|Shuffle (Variables|Default|GetTemp_playlist))
        (Variables|Default|SetTracks_played 0)))))

(event Input|KeyboardEvents|F
  (params (Key :type Key%20Structure :default "None"))
  (:Pressed
    (Audio|Components|Audio|Stop (Variables|Default|GetCurrent_track))))

(fn ConstructionScript)